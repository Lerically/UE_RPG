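; BP_AI_Boss is a boss AI Blueprint that keeps its AI controller informed of the boss's health.
; Each Tick, after the parent logic, it casts its controller to BP_AIControl_General_Boss and copies current and maximum health from the BPCPlayerStates component into it.
; The construction script only calls its parent, and the other events are disabled stubs.
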(event `self.ReceiveTick`
  (params (DeltaSeconds :type "Float (single-precision)"))
  (bind _bpc_playerstates (`self.BPC_PlayerStates`))
  (`parent.ReceiveTick` DeltaSeconds)
  (bind _asbp_aicontrol_general_boss (cast `/Game/AI/Boss/BP_AIControl_General_Boss` (`AIBlueprintHelperLibrary.GetAIController` self)))
  (set `/Game/AI/Boss/BP_AIControl_General_Boss.Health` (`/Game/Blueprint/BPC_PlayerStates.Current Health` _bpc_playerstates) _asbp_aicontrol_general_boss)
  (set `/Game/AI/Boss/BP_AIControl_General_Boss.MaxHealth` (`/Game/Blueprint/BPC_PlayerStates.Max Health` _bpc_playerstates) _asbp_aicontrol_general_boss))

(fn `UserConstructionScript`
  (`parent.UserConstructionScript`))