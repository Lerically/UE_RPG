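; Quest component that tracks the active quest's eliminate-enemy and open-chest objectives and drives a quest HUD widget created at BeginPlay.
; Separate events show the quest name and fill the objective list.
; Enemy kills shrink a shared target array until empty, while chest openings match a specific chest; both mark objectives complete on the HUD.
; Only chest completions advance the counter that plays the quest-completed animation and clears the quest.
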(event `self.ReceiveBeginPlay`
  (bind _returnvalue (`|CreateWidget` "/Game/Quest_System/WB_QuestHUD.WB_QuestHUD_C"))
  (bind _output_get (set `self.QuestHUDWidget` _returnvalue))
  (`UserWidget.AddToViewport` _output_get 0)
  (`/Game/Quest_System/WB_QuestHUD.HideQuestpanel` (`self.QuestHUDWidget`)))

(event `SetActiveQuestText`
  (`TextBlock.SetText` (`/Game/Quest_System/WB_QuestHUD.ActiveQuestText` (`self.QuestHUDWidget`)) (`KismetTextLibrary.Conv_StringToText` (`.Name_2_FEC0DF56434B56609A8AC0B53DCBD59D` (break `/Game/Quest_System/S_Quest` (`self.ActiveQuest`)))))
  (`/Game/Quest_System/WB_QuestHUD.ShowQuestPanel` (`self.QuestHUDWidget`)))

(event `EliminateEnemy`
  (params (`Enemy Elimined` :type "Actor Object Reference"))
  (bind (_activequest_name _activequest_description _activequest_secondary _activequest_completed _activequest_objectives) (break `/Game/Quest_System/S_Quest` (`self.ActiveQuest`)))
  (for _array_element _activequest_objectives
    (bind (_nameaim _completed _actortoeliminate _chesttoopen _iseliminateenemyobjective _ischestobjective) (break `/Game/Quest_System/S_QuestObjective` _array_element))
    (if (and (not _completed) _iseliminateenemyobjective)
      (if (not (!= (`KismetArrayLibrary.Array_Length` (`self.EnemyActorArray`)) 0))
        (bind _output_get (set `self.EnemyActorArray` _actortoeliminate)))
      (`KismetArrayLibrary.Array_RemoveItem` _output_get `Enemy Elimined`)
      (`|VariableSetRef` _array_element (make `/Game/Quest_System/S_QuestObjective` _nameaim false (`self.EnemyActorArray`) _chesttoopen _iseliminateenemyobjective _ischestobjective))
      (if (== (`KismetArrayLibrary.Array_Length` (`self.EnemyActorArray`)) 0)
        (`|VariableSetRef` _array_element (make `/Game/Quest_System/S_QuestObjective` _nameaim true _ _chesttoopen _iseliminateenemyobjective _ischestobjective))
        (`/Game/Quest_System/WB_QuestHUD.CompleteObejective` (`self.QuestHUDWidget`) _array_element)
        (`KismetSystemLibrary.PrintString` "Complete")))))

(event `SetObjective`
  (bind (_activequest_name _activequest_description _activequest_secondary _activequest_completed _activequest_objectives) (break `/Game/Quest_System/S_Quest` (`self.ActiveQuest`)))
  (`/Game/Quest_System/WB_QuestHUD.FillObjectives` (`self.QuestHUDWidget`) _activequest_objectives))

(event `OpenChest`
  (params (Chest :type "Actor Object Reference"))
  (bind (_activequest_name _activequest_description _activequest_secondary _activequest_completed _activequest_objectives) (break `/Game/Quest_System/S_Quest` (`self.ActiveQuest`)))
  (for _array_element _activequest_objectives
    (bind (_nameaim _completed _actortoeliminate _chesttoopen _iseliminateenemyobjective _ischestobjective) (break `/Game/Quest_System/S_QuestObjective` _array_element))
    (if (and _ischestobjective (== Chest _chesttoopen))
      (`|VariableSetRef` _array_element (make `/Game/Quest_System/S_QuestObjective` _activequest_name true _actortoeliminate null _activequest_secondary _activequest_completed))
      (`/Game/Quest_System/WB_QuestHUD.CompleteObejective` (`self.QuestHUDWidget`) _array_element)
      (`self.ObjectiveCompleted`)
      (`KismetSystemLibrary.PrintString` "Complete"))))

(event `ObjectiveCompleted`
  (bind (_activequest_name _activequest_description _activequest_secondary _activequest_completed _activequest_objectives) (break `/Game/Quest_System/S_Quest` (`self.ActiveQuest`)))
  (`/Engine/EditorBlueprintResources/StandardMacros.IncrementInt` (`self.ObjectiveCompeleted`)
    (:`  `
      (if (>= (`self.ObjectiveCompeleted`) (`KismetArrayLibrary.Array_Length` _activequest_objectives))
        (`KismetSystemLibrary.PrintString` "Finished Quest")
        (`/Game/Quest_System/WB_QuestHUD.PlayQuestCompletedAnimation` (`self.QuestHUDWidget`))
        (set `self.ActiveQuest` (struct))
        (set `self.ObjectiveCompeleted` 0)))))