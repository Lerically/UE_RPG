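; Quest giver actor that plays dialogue when interacted with, then opens a quest menu.
; An overlap radius (named AssasinationRadius) shows an interact widget to the player, which Tick rotates toward the camera.
; Repeated Interact calls step through Dialogue lines, then create the quest menu and fill it from Quests.
; The menu receives a back-reference to the giver, and Interact or CloseWidget closes it, restoring game-only input.
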(event `self.ReceiveTick`
  (params (DeltaSeconds :type "Float (single-precision)"))
  ;[0.05098 0.05098 0.05098] Dummy Statement Update
  (`SceneComponent.K2_SetWorldRotation` (`self.InteractWidget`) (`KismetMathLibrary.FindLookAtRotation` (`SceneComponent.K2_GetComponentLocation` (`self.InteractWidget`)) (`SceneComponent.K2_GetComponentLocation` (`PlayerCameraManager.TransformComponent` (`GameplayStatics.GetPlayerCameraManager` 0)))) false false))

(event `self.AssasinationRadius.OnComponentBeginOverlap`
  (params (OverlappedComponent :type "PrimitiveComponent Object Reference") (OtherActor :type "Actor Object Reference") (OtherComp :type "PrimitiveComponent Object Reference") (OtherBodyIndex :type Integer) (bFromSweep :type Boolean) (SweepResult :type "HitResult Structure (by ref)"))
  ;[0.05098 0.05098 0.05098] Assasination Start Detect
  (cast `/Game/ThirdPerson/Blueprints/BP_ThirdPersonCharacter` OtherActor)
  (`SceneComponent.SetVisibility` (`self.InteractWidget`) true false))

(event `self.AssasinationRadius.OnComponentEndOverlap`
  (params (OverlappedComponent :type "PrimitiveComponent Object Reference") (OtherActor :type "Actor Object Reference") (OtherComp :type "PrimitiveComponent Object Reference") (OtherBodyIndex :type Integer))
  ;[0.05098 0.05098 0.05098] Assasination End Detect
  (cast `/Game/ThirdPerson/Blueprints/BP_ThirdPersonCharacter` OtherActor)
  (`SceneComponent.SetVisibility` (`self.InteractWidget`) false false))

(event `/Game/Quest_System/BPI_Quest.Interact`
  (bind _returnvalue (`GameplayStatics.GetPlayerController` 0))
  (bind _returnvalue_2 (`GameplayStatics.GetPlayerController` 0))
  (if (not (`self.WidgetActive`))
    (if (not (`self.DialogueOpened`))
      (bind _returnvalue_3 (`|CreateWidget` "/Game/Quest_System/WB_QuestDialoge.WB_QuestDialoge_C"))
      (bind _output_get (set `self.DialogueWidget` _returnvalue_3))
      (`UserWidget.AddToViewport` _output_get 0)
      (set `self.DialogueOpened` true)
      (`TextBlock.SetText` (`/Game/Quest_System/WB_QuestDialoge.DialogueText` (`self.DialogueWidget`)) (`KismetTextLibrary.Conv_StringToText` (`|GetArrayItem` (`self.Dialogue`) (`self.DialogueIndex`))))
      (`/Engine/EditorBlueprintResources/StandardMacros.IncrementInt` (`self.DialogueIndex`)
        (:`  `
          (set `PlayerController.bShowMouseCursor` true _returnvalue_2)
          (`WidgetBlueprintLibrary.SetInputMode_GameAndUIEx` _returnvalue_2 (`self.Quest Widget`))))
      (else
        (`TextBlock.SetText` (`/Game/Quest_System/WB_QuestDialoge.DialogueText` (`self.DialogueWidget`)) (`KismetTextLibrary.Conv_StringToText` (`|GetArrayItem` (`self.Dialogue`) (`self.DialogueIndex`))))
        (`/Engine/EditorBlueprintResources/StandardMacros.IncrementInt` (`self.DialogueIndex`)
          (:`  `
            (if (> (`self.DialogueIndex`) (`KismetArrayLibrary.Array_Length` (`self.Dialogue`)))
              (`Widget.RemoveFromParent` (`self.DialogueWidget`))
              (set `self.DialogueWidget` null)
              (set `self.DialogueIndex` 0)
              (set `self.DialogueOpened` false)
              (`self.Open Quest Widget`))))))
    (else
      (`Widget.RemoveFromParent` (`self.Quest Widget`) :!label _label)
      (set `self.Quest Widget` null)
      (set `PlayerController.bShowMouseCursor` false _returnvalue)
      (`WidgetBlueprintLibrary.SetInputMode_GameOnly` _returnvalue)
      (set `self.WidgetActive` false))))

(event `CloseWidget`
  (goto _label))

(event `Open Quest Widget`
  (bind _returnvalue (`|CreateWidget` "/Game/Quest_System/WB_QuestMenu.WB_QuestMenu_C"))
  (bind _output_get (set `self.Quest Widget` _returnvalue))
  (`UserWidget.AddToViewport` _output_get 0)
  (set `self.WidgetActive` true)
  (set `/Game/Quest_System/WB_QuestMenu.Quest Giver BP` self (`self.Quest Widget`))
  (for _array_element (`self.quests`)
    (`/Game/Quest_System/WB_QuestMenu.Add Quest` (`self.Quest Widget`) _array_element)))

(fn `UserConstructionScript`)