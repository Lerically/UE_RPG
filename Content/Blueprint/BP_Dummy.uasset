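; BP_Dummy is a target character that takes damage and can be stealth-assassinated from behind.
; An overlap radius toggles the assassinate prompt for the player, and both it and the health bar face the camera on Tick.
; Damage triggers a random hit montage, knockback along player facing and BPCPlayerStates health reduction, ragdolling on death.
; StealthBackAssasin plays the victim montage, schedules delayed ragdoll and returns the attacker's alignment location and rotation.
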(event `self.ReceiveBeginPlay`
  ;[0.05098 0.05098 0.05098] Dummy Health Bar Update Info Source
  (bind _aswb_dummy_hp (cast `/Game/UI/WB_DummyHP` (`WidgetComponent.GetWidget` (`self.HealthBarWidget`))))
  (set `self.healthBarUi` _aswb_dummy_hp))

(event `self.ReceiveTick`
  (params (DeltaSeconds :type "Float (single-precision)"))
  ;[0.05098 0.05098 0.05098] Dummy Statement Update
  (`SceneComponent.K2_SetWorldRotation` (`self.AssasinateWidget`) (`KismetMathLibrary.FindLookAtRotation` (`SceneComponent.K2_GetComponentLocation` (`self.AssasinateWidget`)) (`SceneComponent.K2_GetComponentLocation` (`PlayerCameraManager.TransformComponent` (`GameplayStatics.GetPlayerCameraManager` 0)))) false false)
  (`SceneComponent.K2_SetWorldRotation` (`self.HealthBarWidget`) (`KismetMathLibrary.FindLookAtRotation` (`SceneComponent.K2_GetComponentLocation` (`self.AssasinateWidget`)) (`SceneComponent.K2_GetComponentLocation` (`PlayerCameraManager.TransformComponent` (`GameplayStatics.GetPlayerCameraManager` 0)))) false false))

(event `Ragdoll`
  ;[0.05098 0.05098 0.05098] Ragdoll
  (`|ExecutionSequence`
    (:`then_0`
      (`KismetSystemLibrary.Delay` 2.5)
      (`PrimitiveComponent.SetSimulatePhysics` (`self.Mesh`) true))
    (:`then_1`
      (`KismetSystemLibrary.Delay` 1.7)
      (`GameplayStatics.PlaySoundAtLocation` "/Game/Audio/Grunts-Hits/SC_Death.SC_Death" (`self.K2_GetActorLocation`) (struct) 1.0 1.0 0.0 "/Game/Audio/SA_Character.SA_Character" null null null))))

(event `self.AssasinationRadius.OnComponentBeginOverlap`
  (params (OverlappedComponent :type "PrimitiveComponent Object Reference") (OtherActor :type "Actor Object Reference") (OtherComp :type "PrimitiveComponent Object Reference") (OtherBodyIndex :type Integer) (bFromSweep :type Boolean) (SweepResult :type "HitResult Structure (by ref)"))
  ;[0.05098 0.05098 0.05098] Assasination Start Detect
  (cast `/Game/ThirdPerson/Blueprints/BP_ThirdPersonCharacter` OtherActor)
  (`SceneComponent.SetVisibility` (`self.AssasinateWidget`) true false))

(event `self.AssasinationRadius.OnComponentEndOverlap`
  (params (OverlappedComponent :type "PrimitiveComponent Object Reference") (OtherActor :type "Actor Object Reference") (OtherComp :type "PrimitiveComponent Object Reference") (OtherBodyIndex :type Integer))
  ;[0.05098 0.05098 0.05098] Assasination End Detect
  (cast `/Game/ThirdPerson/Blueprints/BP_ThirdPersonCharacter` OtherActor)
  (`SceneComponent.SetVisibility` (`self.AssasinateWidget`) false false))

(event `self.ReceiveAnyDamage`
  (params (Damage :type "Float (single-precision)") (DamageType :type "DamageType Object Reference") (InstigatedBy :type "Controller Object Reference") (DamageCauser :type "Actor Object Reference"))
  ;[0.05098 0.05098 0.05098] DummyDamageTaking
  (`self.PlayAnimMontage` (`|GetArrayItem` (`self.HitAnims`) (`KismetMathLibrary.RandomIntegerInRange` 0 (- (`KismetArrayLibrary.Array_Length` (`self.HitAnims`)) 1))))
  (bind _asbp_third_person_character (cast `/Game/ThirdPerson/Blueprints/BP_ThirdPersonCharacter` (`GameplayStatics.GetPlayerCharacter` 0)))
  (`self.LaunchCharacter` (* (`KismetMathLibrary.GetForwardVector` (`self.K2_GetActorRotation` _asbp_third_person_character)) 700.0))
  (`GameplayStatics.PlaySoundAtLocation` "/Game/Audio/Grunts-Hits/Death2.Death2" (`self.K2_GetActorLocation`) (struct) 1.0 (`KismetMathLibrary.RandomFloatInRange` -1.5 1.3) 0.0 "/Game/Audio/SA_Character.SA_Character" null null null)
  (bind _isplayerdead (`/Game/Blueprint/BPC_PlayerStates.Decrease Health` (`self.BPC_PlayerStates`) Damage))
  (if _isplayerdead
    (`PrimitiveComponent.SetSimulatePhysics` (`self.Mesh`) true)
    (`GameplayStatics.PlaySoundAtLocation` "/Game/Audio/Grunts-Hits/SC_Death.SC_Death" (`self.K2_GetActorLocation`) (struct) 1.0 1.0 0.0 "/Game/Audio/SA_Character.SA_Character" null null null)
    (`SceneComponent.SetVisibility` (`self.HealthBarWidget`) false false)))

(fn `StealthBackAssasin`
  (returns (REFLocation :type "Vector Structure") (AssasinRotation :type "Rotator Structure"))
  (`self.PlayAnimMontage` "/Game/Characters/RPG_Character/Animations/Assassinations/Paired_Knife_Stealth_KidneyAndNeck_Vic_Montage.Paired_Knife_Stealth_KidneyAndNeck_Vic_Montage")
  (`self.Ragdoll`)
  (`SceneComponent.SetVisibility` (`self.AssasinateWidget`) false false)
  (return (`SceneComponent.K2_GetComponentLocation` (`self.AssasinREF`)) (`self.K2_GetActorRotation`)))

(fn `UserConstructionScript`)