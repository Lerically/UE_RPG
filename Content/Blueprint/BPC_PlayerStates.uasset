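; Actor component that holds health, stamina, XP and level for the player, dummy and AI characters.
; BeginPlay waits a tick, casts the owner to set CharacterType, and fills its bars.
; Damage updates the matching UI via CharacterType selects; other stat functions write only to the player HUD.
; Decrease functions return true on depletion, and enough XP triggers a level-up that raises MaxXP, resets XP and plays sounds.
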(event `self.ReceiveBeginPlay`
  (bind _hud_widget (`/Game/ThirdPerson/Blueprints/BP_ThirdPersonCharacter.HUD Widget` (`self.PlayerREF`)))
  (`KismetSystemLibrary.DelayUntilNextTick`)
  (bind _asbp_third_person_character (cast `/Game/ThirdPerson/Blueprints/BP_ThirdPersonCharacter` (`self.GetOwner`))
    (:`then`
      (set `self.PlayerREF` _asbp_third_person_character)
      (set `self.isPlayer` true)
      (`ProgressBar.SetPercent` (`/Game/UI/WB_HUD.StaminaBar` (`/Game/ThirdPerson/Blueprints/BP_ThirdPersonCharacter.HUD Widget` (`self.PlayerREF`))) (/ (`self.Current Stamina`) (`self.Max Stamina`)))
      (set `self.CharacterType` "NewEnumerator0"))
    (:`CastFailed`
      (bind _asbp_dummy (cast `/Game/Blueprint/BP_Dummy` (`self.GetOwner`))
        (:`then`
          (set `self.DummyRef` _asbp_dummy)
          (set `self.isPlayer` false)
          (set `self.CharacterType` "NewEnumerator1"))
        (:`CastFailed`
          (bind _asbp_ai (cast `/Game/AI/BP_AI` (`self.GetOwner`)))
          (set `self.AI BP` _asbp_ai)
          (set `self.CharacterType` "NewEnumerator2")))))
  (`ProgressBar.SetPercent` (select `/Game/Blueprint/E_CharacterType` (`self.CharacterType`) :`NewEnumerator0` (`/Game/UI/WB_HUD.HealthBar` (`/Game/ThirdPerson/Blueprints/BP_ThirdPersonCharacter.HUD Widget` (`self.PlayerREF`))) :`NewEnumerator1` (`/Game/UI/WB_DummyHP.HealthBar` (`/Game/Blueprint/BP_Dummy.healthBarUi` (`self.DummyRef`))) :`NewEnumerator2` (`/Game/UI/WB_DummyHP.HealthBar` (`/Game/AI/BP_AI.healthBarUi` (`self.AI BP`)))) (/ (`self.Current Health`) (`self.Max Health`)))
  (`TextBlock.SetText` (select `/Game/Blueprint/E_CharacterType` (`self.CharacterType`) :`NewEnumerator0` (`/Game/UI/WB_HUD.HealthText` (`/Game/ThirdPerson/Blueprints/BP_ThirdPersonCharacter.HUD Widget` (`self.PlayerREF`))) :`NewEnumerator1` (`/Game/UI/WB_DummyHP.HealthText` (`/Game/Blueprint/BP_Dummy.healthBarUi` (`self.DummyRef`))) :`NewEnumerator2` (`/Game/UI/WB_DummyHP.HealthText` (`/Game/AI/BP_AI.healthBarUi` (`self.AI BP`)))) (`KismetTextLibrary.Conv_DoubleToText` (`self.Current Health`) "HalfToEven"))
  (if (`self.isPlayer`)
    (`ProgressBar.SetPercent` (`/Game/UI/WB_HUD.XP_Bar` _hud_widget) (/ (`self.XP`) (`self.Max XP`)))
    (`TextBlock.SetText` (`/Game/UI/WB_HUD.XP_Container` _hud_widget) (`|FormatText` "{Current XP} / {Max XP}" (`self.XP`) (`self.Max XP`)))
    (`TextBlock.SetText` (`/Game/UI/WB_HUD.LevelText` (`/Game/ThirdPerson/Blueprints/BP_ThirdPersonCharacter.HUD Widget` (`self.PlayerREF`))) (`KismetTextLibrary.Conv_IntToText` (`self.Level`)))))

(fn `Decrease Health`
  (params (Damage :type "Float (double-precision)"))
  (returns (isPlayerDead :type Boolean))
  (if (not (<= (`self.Current Health`) 0.0))
    (bind _output_get (set `self.Current Health` (- (`self.Current Health`) Damage)))
    (`ProgressBar.SetPercent` (select `/Game/Blueprint/E_CharacterType` (`self.CharacterType`) :`NewEnumerator0` (`/Game/UI/WB_HUD.HealthBar` (`/Game/ThirdPerson/Blueprints/BP_ThirdPersonCharacter.HUD Widget` (`self.PlayerREF`))) :`NewEnumerator1` (`/Game/UI/WB_DummyHP.HealthBar` (`/Game/Blueprint/BP_Dummy.healthBarUi` (`self.DummyRef`))) :`NewEnumerator2` (`/Game/UI/WB_DummyHP.HealthBar` (`/Game/AI/BP_AI.healthBarUi` (`self.AI BP`)))) (/ _output_get (`self.Max Health`)))
    (`TextBlock.SetText` (select `/Game/Blueprint/E_CharacterType` (`self.CharacterType`) :`NewEnumerator0` (`/Game/UI/WB_HUD.HealthText` (`/Game/ThirdPerson/Blueprints/BP_ThirdPersonCharacter.HUD Widget` (`self.PlayerREF`))) :`NewEnumerator1` (`/Game/UI/WB_DummyHP.HealthText` (`/Game/Blueprint/BP_Dummy.healthBarUi` (`self.DummyRef`))) :`NewEnumerator2` (`/Game/UI/WB_DummyHP.HealthText` (`/Game/AI/BP_AI.healthBarUi` (`self.AI BP`)))) (`KismetTextLibrary.Conv_DoubleToText` (`self.Current Health`) "HalfToEven"))
    (if (<= (`self.Current Health`) 0.0)
      _
      (else
        (return false))))
  (return true))

(fn `Decrease Stamina`
  (params (`Stamina Depleted` :type "Float (double-precision)"))
  (returns (`No StaminaLeft` :type Boolean))
  (if (not (<= (`self.Current Stamina`) 0.0))
    (set `self.Current Stamina` (- (`self.Current Stamina`) `Stamina Depleted`))
    (`ProgressBar.SetPercent` (`/Game/UI/WB_HUD.StaminaBar` (`/Game/ThirdPerson/Blueprints/BP_ThirdPersonCharacter.HUD Widget` (`self.PlayerREF`))) (/ (`self.Current Stamina`) (`self.Max Stamina`)))
    (if (<= (`self.Current Stamina`) 0.0)
      _
      (else
        (return false))))
  (return true))

(fn `Increase Health`
  (params (`Added Health` :type "Float (double-precision)"))
  (bind _hud_widget (`/Game/ThirdPerson/Blueprints/BP_ThirdPersonCharacter.HUD Widget` (`self.PlayerREF`)))
  (set `self.Current Health` (+ (`self.Current Health`) `Added Health`))
  (if (> (`self.Current Health`) (`self.Max Health`))
    (set `self.Current Health` (`self.Max Health`)))
  (`ProgressBar.SetPercent` (`/Game/UI/WB_HUD.HealthBar` _hud_widget) (/ (`self.Current Health`) (`self.Max Health`)))
  (`TextBlock.SetText` (`/Game/UI/WB_HUD.HealthText` _hud_widget) (`KismetTextLibrary.Conv_DoubleToText` (`self.Current Health`) "HalfToEven")))

(fn `Increase Level`
  (params (`Added Level` :type Integer))
  (set `self.Level` (+ (`self.Level`) `Added Level`))
  (set `self.Max XP` (+ (`self.Max XP`) 40.0))
  (set `self.XP` 0.0)
  (`TextBlock.SetText` (`/Game/UI/WB_HUD.LevelText` (`/Game/ThirdPerson/Blueprints/BP_ThirdPersonCharacter.HUD Widget` (`self.PlayerREF`))) (`KismetTextLibrary.Conv_IntToText` (`self.Level`)))
  (`GameplayStatics.PlaySound2D` "/Game/Audio/UI/LevelUp1.LevelUp1" 1.0 1.0 0.0 null null)
  (`GameplayStatics.PlaySound2D` "/Game/Audio/UI/LevelUp2.LevelUp2" 1.0 1.0 0.0 null null))

(fn `Increase Max Health`
  (params (`Health Incremention` :type "Float (double-precision)"))
  (bind _hud_widget (`/Game/ThirdPerson/Blueprints/BP_ThirdPersonCharacter.HUD Widget` (`self.PlayerREF`)))
  (set `self.Max Health` (+ (`self.Max Health`) `Health Incremention`))
  (`ProgressBar.SetPercent` (`/Game/UI/WB_HUD.HealthBar` _hud_widget) (/ (`self.Current Health`) (`self.Max Health`)))
  (`TextBlock.SetText` (`/Game/UI/WB_HUD.HealthText` _hud_widget) (`KismetTextLibrary.Conv_DoubleToText` (`self.Current Health`) "HalfToEven")))

(fn `Increase Max Stamina`
  (params (AddedStamina :type "Float (double-precision)"))
  (set `self.Max Stamina` (+ (`self.Max Stamina`) AddedStamina))
  (`ProgressBar.SetPercent` (`/Game/UI/WB_HUD.StaminaBar` (`/Game/ThirdPerson/Blueprints/BP_ThirdPersonCharacter.HUD Widget` (`self.PlayerREF`))) (/ (`self.Current Stamina`) (`self.Max Stamina`))))

(fn `Increase Stamina`
  (params (`Added Stamina` :type "Float (double-precision)"))
  (set `self.Current Stamina` (+ (`self.Current Stamina`) `Added Stamina`))
  (if (> (`self.Current Stamina`) (`self.Max Stamina`))
    (set `self.Current Stamina` (`self.Max Stamina`)))
  (`ProgressBar.SetPercent` (`/Game/UI/WB_HUD.StaminaBar` (`/Game/ThirdPerson/Blueprints/BP_ThirdPersonCharacter.HUD Widget` (`self.PlayerREF`))) (/ (`self.Current Stamina`) (`self.Max Stamina`))))

(fn `Increase XP`
  (params (`Added XP` :type "Float (double-precision)"))
  (set `self.XP` (+ (`self.XP`) `Added XP`))
  (if (>= (`self.XP`) (`self.Max XP`))
    (`self.Increase Level` 1))
  (`ProgressBar.SetPercent` (`/Game/UI/WB_HUD.XP_Bar` (`/Game/ThirdPerson/Blueprints/BP_ThirdPersonCharacter.HUD Widget` (`self.PlayerREF`))) (/ (`self.XP`) (`self.Max XP`)))
  (`TextBlock.SetText` (`/Game/UI/WB_HUD.XP_Container` (`/Game/ThirdPerson/Blueprints/BP_ThirdPersonCharacter.HUD Widget` (`self.PlayerREF`))) (`|FormatText` "{Current XP} / {Max XP}" (`self.XP`) (`self.Max XP`))))